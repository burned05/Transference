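; Level actor for a platform that shuttles back and forth between two markers, with a SwitchActivate event to start it.
; While Ready is false, Tick moves the Cube by lerping between RightMove and LeftMove, stepping Alpha by delta time over TimeToMovePlatform.
; MovingRight flips at each end for continuous ping-pong motion.
; Naming is inverted: SwitchActivate clears Ready to enable movement, and MovingRight travels toward LeftMove.
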(event Custom|Move_Platform_Right
  (bind _output_get (Variables|Default|SetAlpha (+ (Variables|Default|GetAlpha) (/ (Utilities|Time|GetWorldDeltaSeconds) (Variables|Default|GetTimeToMovePlatform)))))
  (Transformation|SetWorldLocation (Variables|Default|GetCube) (Math|Vector|Lerp(Vector) (Transformation|GetWorldLocation (Variables|Default|GetRightMove)) (Transformation|GetWorldLocation (Variables|Default|GetLeftMove)) (Variables|Default|GetAlpha)) false false)
  (if (>= _output_get 1.0)
    (Variables|Default|SetMovingRight false)))

(event Custom|Move_Platform_Left
  (bind _output_get (Variables|Default|SetAlpha (- (Variables|Default|GetAlpha) (/ (Utilities|Time|GetWorldDeltaSeconds) (Variables|Default|GetTimeToMovePlatform)))))
  (Transformation|SetWorldLocation (Variables|Default|GetCube) (Math|Vector|Lerp(Vector) (Transformation|GetWorldLocation (Variables|Default|GetRightMove)) (Transformation|GetWorldLocation (Variables|Default|GetLeftMove)) (Variables|Default|GetAlpha)) false false)
  (if (<= _output_get 0.0)
    (Variables|Default|SetMovingRight true)))

(event EventBeginPlay
  (|CallParentFunction) ; This node is disabled and will not be called.\nDrag off pins to build functionality.
)

(event Collision|EventActorBeginOverlap
  (params (OtherActor :type Actor%20Object%20Reference))
  (|CallParentFunction OtherActor) ; This node is disabled and will not be called.\nDrag off pins to build functionality.
)

(event EventSwitchActivate
  (Variables|Default|SetReady false))

(event EventTick
  (params (DeltaSeconds :type Float%20%28single-precision%29))
  (if (not (Variables|Default|GetReady))
    (if (Variables|Default|GetMovingRight)
      (CallFunction|MovePlatformRight)
      (else
        (CallFunction|MovePlatformLeft)))))

(fn ConstructionScript
  (|CallParentFunction))