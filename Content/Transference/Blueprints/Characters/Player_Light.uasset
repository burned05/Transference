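; Player_Light is a playable character Blueprint whose Action event drives jumping.
; Pressing triggers Jump and, if the character is not already airborne, spawns a scaled-down explosion emitter and plays a jump sound at FireSpot; releasing stops the jump.
; The airborne check reads IsInAir from the Player_Light_Anim_BP animation instance rather than from the movement component.
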(event EventBeginPlay
  (|CallParentFunction) ; This node is disabled and will not be called.\nDrag off pins to build functionality.
)

(event Collision|EventActorBeginOverlap
  (params (OtherActor :type Actor%20Object%20Reference))
  (|CallParentFunction OtherActor) ; This node is disabled and will not be called.\nDrag off pins to build functionality.
)

(event EventAction
  (params (Pressed :type Boolean))
  (bind _firespot (Variables|Default|GetFireSpot))
  (if Pressed
    (Character|Jump)
    (bind _inair (Utilities|IsinAir)
      (:out
        (if (not _inair)
          (Effects|SpawnEmitterAttached "/Game/StarterContent/Particles/P_Explosion.P_Explosion" _firespot "None" "0, 0, 0" "0, 0, 0" "0.300000,0.300000,0.300000")
          (Audio|PlaySoundatLocation "/Game/Transference/Sound/SFX/Jump_Light.Jump_Light" (Transformation|GetWorldLocation _firespot)))))
    (else
      (Character|StopJumping))))

(event EventTick
  (params (DeltaSeconds :type Float%20%28single-precision%29))
  (|CallParentFunction DeltaSeconds) ; This node is disabled and will not be called.\nDrag off pins to build functionality.
)

(fn ConstructionScript
  (|CallParentFunction))