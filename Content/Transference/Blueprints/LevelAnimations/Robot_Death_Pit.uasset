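; Level death-pit trap for the heavy robot, with a saw blade that rotates on every Tick.
; The first Player_Heavy to enter the box reveals a physics-simulated Heavy stand-in and shifts the fake walk floor.
; The real pawn is teleported to a marker component, and player controller 0 calls PossessDefault.
; A Triggered flag makes it one-shot; an AddForce push on the stand-in is left unconnected.
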(event OnComponentBeginOverlap(Box)
  (params (OverlappedComponent :type Primitive%20Component%20Object%20Reference) (OtherActor :type Actor%20Object%20Reference) (OtherComp :type Primitive%20Component%20Object%20Reference) (OtherBodyIndex :type Integer) (bFromSweep :type Boolean) (SweepResult :type Hit%20Result%20Structure%20%28by%20ref%29))
  (if (not (Variables|Default|Gettriggered))
    (bind _asplayer_heavy (Utilities|Casting|CastToPlayer_Heavy OtherActor))
    (Rendering|SetVisibility (Variables|Default|GetHeavy) true false)
    (Physics|SetSimulatePhysics (Variables|Default|GetHeavy) true)
    (Transformation|SetRelativeLocation (Variables|Default|GetFakeWalkFloor) "-30.000000,-5.000000,190.000000" false false)
    (Transformation|SetActorLocation _asplayer_heavy (Transformation|GetWorldLocation (Variables|Default|GetTeleport)) false false)
    (Variables|Default|Settriggered true)
    (bind _asplayer_controller_base (Utilities|Casting|CastToPlayer_Controller_Base (Game|GetPlayerController 0)))
    (Default|PossessDefault _asplayer_controller_base)))

(event Custom|Spinning_Saw
  (Transformation|AddLocalRotation (Variables|Default|GetSawBlade) (Math|Rotator|MakeRotator (+ (Variables|Default|GetBladeSpeed) 1.0) 0.0 0.0) false false))

(event EventBeginPlay
  (|CallParentFunction) ; This node is disabled and will not be called.\nDrag off pins to build functionality.
)

(event Collision|EventActorBeginOverlap
  (params (OtherActor :type Actor%20Object%20Reference))
  (|CallParentFunction OtherActor) ; This node is disabled and will not be called.\nDrag off pins to build functionality.
)

(event EventTick
  (params (DeltaSeconds :type Float%20%28single-precision%29))
  (CallFunction|SpinningSaw))

(fn ConstructionScript
  (|CallParentFunction))