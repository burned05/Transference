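; Level 1 elevator actor that rises once a switch activates it.
; SwitchActivate sets a moving flag and clears Ready, so Tick runs the move-up logic each frame.
; That logic spins two screw components and lerps the platform between down and up marker components over TimeToMoveElevator.
; At the top it stops and sets Ready; there is no descent or alpha reset.
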(event Custom|Move_Elevator_Up
  (CallFunction|RotateScrews)
  (bind _output_get (Variables|Default|SetAlpha (+ (Variables|Default|GetAlpha) (/ (Utilities|Time|GetWorldDeltaSeconds) (Variables|Default|GetTimeToMoveElevator)))))
  (Transformation|SetWorldLocation (Variables|Default|GetElevator) (Math|Vector|Lerp(Vector) (Transformation|GetWorldLocation (Variables|Default|GetElevatorDown)) (Transformation|GetWorldLocation (Variables|Default|GetElevatorUp)) (Variables|Default|GetAlpha)) false false)
  (if (>= _output_get 1.0)
    (Variables|Default|SetReady true)
    (Variables|Default|SetElevator_Moving false)))

(event Custom|RotateScrews
  (Transformation|AddWorldRotation (Variables|Default|GetLeft_Screw) (Math|Rotator|MakeRotator 0.0 0.0 (* (Utilities|Time|GetWorldDeltaSeconds) 1.2e+02)) false false))

(event EventBeginPlay)

(event Collision|EventActorBeginOverlap
  (params (OtherActor :type Actor%20Object%20Reference)))

(event EventTick
  (params (DeltaSeconds :type Float%20%28single-precision%29))
  (if (Variables|Default|GetElevator_Moving)
    (CallFunction|MoveElevatorUp)))

(event EventSwitchActivate
  (Variables|Default|SetElevator_Moving true)
  (Variables|Default|SetReady false))

(fn ConstructionScript)