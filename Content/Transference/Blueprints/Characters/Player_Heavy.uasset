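; Heavy player character Blueprint that picks up, carries and drops Moveable_Object_Physx objects.
; An Action press, accepted only when the forward vector's X is near zero (facing along world Y), releases the held object or sphere-traces ahead for a physics body to grab.
; A PhysicsHandle follows GrabLocation every Tick, and grab or release updates the carrying state in Player_Heavy_Anim_BP.
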(event EventBeginPlay)

(event Collision|EventActorBeginOverlap
  (params (OtherActor :type Actor%20Object%20Reference)))

(event EventTick
  (params (DeltaSeconds :type Float%20%28single-precision%29))
  (bind _grablocation (Variables|Default|GetGrabLocation))
  (Class|PhysicsHandleComponent|SetTargetLocationandRotation (Variables|Default|GetPhysicsHandle) (Transformation|GetWorldLocation _grablocation) (Transformation|GetWorldRotation _grablocation)))

(event EventAction
  (params (Pressed :type Boolean))
  (bind _returnvalue (Transformation|GetActorRotation))
  (bind _returnvalue_2 (Transformation|GetActorLocation))
  (bind _returnvalue_3 (Math|Rotator|GetRotationXVector _returnvalue))
  (bind _x (Math|Vector|BreakVector _returnvalue_3))
  (if Pressed
    (if (or (Math|Float|NearlyEqual(Float) _x 0.0 1e-06) (Math|Float|NearlyEqual(Float) _x -1.8e+02 1e-06))
      (Utilities|IsValid (Variables|Default|GetHeldObject)
        (:Is%20Valid
          (Physics|Components|PhysicsHandle|ReleaseComponent (Variables|Default|GetPhysicsHandle))
          (Variables|Default|SetHeldObject 0)
          (bind _asplayer_heavy_anim_bp (Utilities|Casting|CastToPlayer_Heavy_Anim_BP (Components|SkeletalMesh|GetAnimInstance (Variables|Character|GetMesh))))
          (Default|SetCarrying _asplayer_heavy_anim_bp false))
        (:Is%20Not%20Valid
          (bind _outhit (Collision|SphereTraceForObjects _returnvalue_2 (+ _returnvalue_2 (* (Transformation|GetActorForwardVector) 5e+01)) 5e+01 (Utilities|Array|MakeArray "ObjectTypeQuery4") false 0 "None"))
          (bind _asmoveable_object_physx (Utilities|Casting|CastToMoveable_Object_Physx (.HitActor (Collision|BreakHitResult _outhit))))
          (Variables|Default|SetHeldObject _asmoveable_object_physx)
          (Physics|Components|PhysicsHandle|GrabComponentatLocationwithRotation (Variables|Default|GetPhysicsHandle) (.HitComponent (Collision|BreakHitResult _outhit)) "None" (Transformation|GetWorldLocation (Variables|/Game/Transference/Blueprints/Objects/Moveable_Object_Physx.Moveable_Object_Physx_C|GetDefaultSceneComponent _asmoveable_object_physx)) (Transformation|GetWorldRotation (Variables|Default|GetGrabLocation)))
          (bind _asplayer_heavy_anim_bp_2 (Utilities|Casting|CastToPlayer_Heavy_Anim_BP (Components|SkeletalMesh|GetAnimInstance (Variables|Character|GetMesh))))
          (Default|SetCarrying _asplayer_heavy_anim_bp_2 true))))))

(fn ConstructionScript
  (|CallParentFunction))